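; Procedural modular building that assembles itself from static mesh tiles in the Construction Script, sized by XSize, YSize and ZFloors.
; Each floor gets four walls and corners, placed by mesh bounds, with door columns using alternate meshes.
; Ground and upper floors use fixed array slots; others share an unseeded random variant per floor, re-rolled on construction.
; Roof edges follow, then a grid of top tiles scaled by column and row.
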(event EventBeginPlay)

(event Collision|EventActorBeginOverlap
  (params (OtherActor :type Actor%20Object%20Reference)))

(event EventTick
  (params (DeltaSeconds :type Float%20%28single-precision%29)))

(fn ConstructionScript
  (bind _corner_meshes (Variables|Meshes|GetCorner%20Meshes))
  (bind _returnvalue (Utilities|Array|LastIndex _corner_meshes))
  (Utilities|FlowControl|Sequence
    (:then_0
      (for _index (range 1 (Variables|BuildingSize|GetZ%20Floors))
        (bind _output_get (Variables|BuildingSize|SetZ%20Current _index))
        (Variables|BuildingSize|SetCurrent%20Height (Math|Float|SelectFloat 0.0 (+ (Variables|BuildingSize|GetCurrent%20Height) (Variables|TilesDimentions|GetWall%20Tile%20Height)) (== _output_get 1)))
        (Variables|BuildingSize|SetRandom%20Floor (Math|Random|RandomIntegerinRange 1 2))
        (Utilities|FlowControl|Sequence
          (:then_0
            ;[1 1 1] X Front
            (for _index_2 (range 1 (Variables|BuildingSize|GetX%20Size))
              (Variables|BuildingSize|SetX%20Current _index_2)
              (Utilities|FlowControl|Sequence
                (:then_0
                  (Variables|BuildingSize|SetCurrent%20X%20Length (+ (Variables|BuildingSize|GetCurrent%20X%20Length) (Variables|TilesDimentions|GetWall%20Tile%20Length))))
                (:then_1
                  (bind _output_get_2 (Variables|Meshes|SetTile (Utilities|Array|Get(acopy) (select (Utilities|Array|ContainsItem (Variables|DoorsPlacement|GetX%20Door%20Places) (Variables|BuildingSize|GetX%20Current)) (Variables|Meshes|GetWall%202%20Meshes) (Variables|Meshes|GetWall%20Meshes)) (Math|Integer|SelectInt 0 (Math|Integer|SelectInt (Utilities|Array|LastIndex (select (Utilities|Array|ContainsItem (Variables|DoorsPlacement|GetX%20Door%20Places) (Variables|BuildingSize|GetX%20Current)) (Variables|Meshes|GetWall%202%20Meshes) (Variables|Meshes|GetWall%20Meshes))) (Math|Integer|SelectInt (- (Utilities|Array|LastIndex (select (Utilities|Array|ContainsItem (Variables|DoorsPlacement|GetX%20Door%20Places) (Variables|BuildingSize|GetX%20Current)) (Variables|Meshes|GetWall%202%20Meshes) (Variables|Meshes|GetWall%20Meshes))) 1) (Math|Integer|SelectInt (- (Utilities|Array|LastIndex (select (Utilities|Array|ContainsItem (Variables|DoorsPlacement|GetX%20Door%20Places) (Variables|BuildingSize|GetX%20Current)) (Variables|Meshes|GetWall%202%20Meshes) (Variables|Meshes|GetWall%20Meshes))) 2) (Math|Integer|SelectInt (- (Utilities|Array|LastIndex (select (Utilities|Array|ContainsItem (Variables|DoorsPlacement|GetX%20Door%20Places) (Variables|BuildingSize|GetX%20Current)) (Variables|Meshes|GetWall%202%20Meshes) (Variables|Meshes|GetWall%20Meshes))) 3) (Math|Integer|SelectInt (- (Utilities|Array|LastIndex (select (Utilities|Array|ContainsItem (Variables|DoorsPlacement|GetX%20Door%20Places) (Variables|BuildingSize|GetX%20Current)) (Variables|Meshes|GetWall%202%20Meshes) (Variables|Meshes|GetWall%20Meshes))) 3) (Math|Integer|SelectInt (- (Utilities|Array|LastIndex (select (Utilities|Array|ContainsItem (Variables|DoorsPlacement|GetX%20Door%20Places) (Variables|BuildingSize|GetX%20Current)) (Variables|Meshes|GetWall%202%20Meshes) (Variables|Meshes|GetWall%20Meshes))) 4) (Variables|BuildingSize|GetRandom%20Floor) (== (Variables|BuildingSize|GetZ%20Current) (- (Variables|BuildingSize|GetZ%20Floors) 4))) (== (Variables|BuildingSize|GetZ%20Current) (- (Variables|BuildingSize|GetZ%20Floors) 3))) (== (Variables|BuildingSize|GetZ%20Current) (- (Variables|BuildingSize|GetZ%20Floors) 3))) (== (Variables|BuildingSize|GetZ%20Current) (- (Variables|BuildingSize|GetZ%20Floors) 2))) (== (Variables|BuildingSize|GetZ%20Current) (- (Variables|BuildingSize|GetZ%20Floors) 1))) (== (Variables|BuildingSize|GetZ%20Current) (Variables|BuildingSize|GetZ%20Floors))) (== (Variables|BuildingSize|GetZ%20Current) 1)))))
                  (Variables|TilesDimentions|SetWall%20Tile%20Length (.x (.max (StaticMesh|GetBoundingBox _output_get_2))))
                  (Variables|TilesDimentions|SetWall%20Tile%20Height (.z (.max (StaticMesh|GetBoundingBox _output_get_2))))
                  (bind _returnvalue_2 (AddComponent|AddStaticMeshComponent false (Math|Transform|MakeTransform (Math|Vector|MakeVector (Variables|BuildingSize|GetCurrent%20X%20Length) 0.0 (Variables|BuildingSize|GetCurrent%20Height)) "0, 0, 0" "1.000000,1.000000,1.000000")))
                  (Components|StaticMesh|SetStaticMesh _returnvalue_2 (Variables|Meshes|GetTile)))))
            (Variables|BuildingSize|SetFinal%20X%20Length (+ (Variables|BuildingSize|GetCurrent%20X%20Length) (Variables|TilesDimentions|GetWall%20Tile%20Length)))
            (Variables|BuildingSize|SetCurrent%20X%20Length 0.0)
            (Variables|TilesDimentions|SetWall%20Tile%20Length 0.0))
          (:then_1
            ;[1 1 1] Y
            (for _index_3 (range 1 (Variables|BuildingSize|GetY%20Size))
              (Variables|BuildingSize|SetY%20Current _index_3)
              (Utilities|FlowControl|Sequence
                (:then_0
                  (Variables|BuildingSize|SetCurrent%20Y%20Length (+ (Variables|BuildingSize|GetCurrent%20Y%20Length) (Variables|TilesDimentions|GetWall%20Tile%20Length))))
                (:then_1
                  (bind _output_get_3 (Variables|Meshes|SetTile (Utilities|Array|Get(acopy) (select (Utilities|Array|ContainsItem (Variables|DoorsPlacement|GetY%20Door%20Places) (Variables|BuildingSize|GetY%20Current)) (Variables|Meshes|GetWall%202%20Meshes) (Variables|Meshes|GetWall%20Meshes)) (Math|Integer|SelectInt 0 (Math|Integer|SelectInt (Utilities|Array|LastIndex (select (Utilities|Array|ContainsItem (Variables|DoorsPlacement|GetY%20Door%20Places) (Variables|BuildingSize|GetY%20Current)) (Variables|Meshes|GetWall%202%20Meshes) (Variables|Meshes|GetWall%20Meshes))) (Math|Integer|SelectInt (- (Utilities|Array|LastIndex (select (Utilities|Array|ContainsItem (Variables|DoorsPlacement|GetY%20Door%20Places) (Variables|BuildingSize|GetY%20Current)) (Variables|Meshes|GetWall%202%20Meshes) (Variables|Meshes|GetWall%20Meshes))) 1) (Math|Integer|SelectInt (- (Utilities|Array|LastIndex (select (Utilities|Array|ContainsItem (Variables|DoorsPlacement|GetY%20Door%20Places) (Variables|BuildingSize|GetY%20Current)) (Variables|Meshes|GetWall%202%20Meshes) (Variables|Meshes|GetWall%20Meshes))) 2) (Math|Integer|SelectInt (- (Utilities|Array|LastIndex (select (Utilities|Array|ContainsItem (Variables|DoorsPlacement|GetY%20Door%20Places) (Variables|BuildingSize|GetY%20Current)) (Variables|Meshes|GetWall%202%20Meshes) (Variables|Meshes|GetWall%20Meshes))) 3) (Math|Integer|SelectInt (- (Utilities|Array|LastIndex (select (Utilities|Array|ContainsItem (Variables|DoorsPlacement|GetY%20Door%20Places) (Variables|BuildingSize|GetY%20Current)) (Variables|Meshes|GetWall%202%20Meshes) (Variables|Meshes|GetWall%20Meshes))) 3) (Math|Integer|SelectInt (- (Utilities|Array|LastIndex (select (Utilities|Array|ContainsItem (Variables|DoorsPlacement|GetY%20Door%20Places) (Variables|BuildingSize|GetY%20Current)) (Variables|Meshes|GetWall%202%20Meshes) (Variables|Meshes|GetWall%20Meshes))) 4) (Variables|BuildingSize|GetRandom%20Floor) (== (Variables|BuildingSize|GetZ%20Current) (- (Variables|BuildingSize|GetZ%20Floors) 4))) (== (Variables|BuildingSize|GetZ%20Current) (- (Variables|BuildingSize|GetZ%20Floors) 3))) (== (Variables|BuildingSize|GetZ%20Current) (- (Variables|BuildingSize|GetZ%20Floors) 3))) (== (Variables|BuildingSize|GetZ%20Current) (- (Variables|BuildingSize|GetZ%20Floors) 2))) (== (Variables|BuildingSize|GetZ%20Current) (- (Variables|BuildingSize|GetZ%20Floors) 1))) (== (Variables|BuildingSize|GetZ%20Current) (Variables|BuildingSize|GetZ%20Floors))) (== (Variables|BuildingSize|GetZ%20Current) 1)))))
                  (Variables|TilesDimentions|SetWall%20Tile%20Length (.x (.max (StaticMesh|GetBoundingBox _output_get_3))))
                  (Variables|TilesDimentions|SetWall%20Tile%20Height (.z (.max (StaticMesh|GetBoundingBox _output_get_3))))
                  (bind _returnvalue_3 (AddComponent|AddStaticMeshComponent false (Math|Transform|MakeTransform (Math|Vector|MakeVector 0.0 (- (* (Variables|BuildingSize|GetCurrent%20Y%20Length) -1.0) (Variables|TilesDimentions|GetWall%20Tile%20Length)) (Variables|BuildingSize|GetCurrent%20Height)) "0.000000,90.000000,0.000000" "1.000000,1.000000,1.000000")))
                  (Components|StaticMesh|SetStaticMesh _returnvalue_3 (Variables|Meshes|GetTile)))
                (:then_2
                  (bind _output_get_4 (Variables|Meshes|SetTile (Utilities|Array|Get(acopy) (select (Utilities|Array|ContainsItem (Variables|DoorsPlacement|GetY%20Door%20Places) (Variables|BuildingSize|GetY%20Current)) (Variables|Meshes|GetWall%202%20Meshes) (Variables|Meshes|GetWall%20Meshes)) (Math|Integer|SelectInt 0 (Math|Integer|SelectInt (Utilities|Array|LastIndex (select (Utilities|Array|ContainsItem (Variables|DoorsPlacement|GetY%20Door%20Places) (Variables|BuildingSize|GetY%20Current)) (Variables|Meshes|GetWall%202%20Meshes) (Variables|Meshes|GetWall%20Meshes))) (Math|Integer|SelectInt (- (Utilities|Array|LastIndex (select (Utilities|Array|ContainsItem (Variables|DoorsPlacement|GetY%20Door%20Places) (Variables|BuildingSize|GetY%20Current)) (Variables|Meshes|GetWall%202%20Meshes) (Variables|Meshes|GetWall%20Meshes))) 1) (Math|Integer|SelectInt (- (Utilities|Array|LastIndex (select (Utilities|Array|ContainsItem (Variables|DoorsPlacement|GetY%20Door%20Places) (Variables|BuildingSize|GetY%20Current)) (Variables|Meshes|GetWall%202%20Meshes) (Variables|Meshes|GetWall%20Meshes))) 2) (Math|Integer|SelectInt (- (Utilities|Array|LastIndex (select (Utilities|Array|ContainsItem (Variables|DoorsPlacement|GetY%20Door%20Places) (Variables|BuildingSize|GetY%20Current)) (Variables|Meshes|GetWall%202%20Meshes) (Variables|Meshes|GetWall%20Meshes))) 3) (Math|Integer|SelectInt (- (Utilities|Array|LastIndex (select (Utilities|Array|ContainsItem (Variables|DoorsPlacement|GetY%20Door%20Places) (Variables|BuildingSize|GetY%20Current)) (Variables|Meshes|GetWall%202%20Meshes) (Variables|Meshes|GetWall%20Meshes))) 3) (Math|Integer|SelectInt (- (Utilities|Array|LastIndex (select (Utilities|Array|ContainsItem (Variables|DoorsPlacement|GetY%20Door%20Places) (Variables|BuildingSize|GetY%20Current)) (Variables|Meshes|GetWall%202%20Meshes) (Variables|Meshes|GetWall%20Meshes))) 4) (Variables|BuildingSize|GetRandom%20Floor) (== (Variables|BuildingSize|GetZ%20Current) (- (Variables|BuildingSize|GetZ%20Floors) 4))) (== (Variables|BuildingSize|GetZ%20Current) (- (Variables|BuildingSize|GetZ%20Floors) 3))) (== (Variables|BuildingSize|GetZ%20Current) (- (Variables|BuildingSize|GetZ%20Floors) 3))) (== (Variables|BuildingSize|GetZ%20Current) (- (Variables|BuildingSize|GetZ%20Floors) 2))) (== (Variables|BuildingSize|GetZ%20Current) (- (Variables|BuildingSize|GetZ%20Floors) 1))) (== (Variables|BuildingSize|GetZ%20Current) (Variables|BuildingSize|GetZ%20Floors))) (== (Variables|BuildingSize|GetZ%20Current) 1)))))
                  (Variables|TilesDimentions|SetWall%20Tile%20Length (.x (.max (StaticMesh|GetBoundingBox _output_get_4))))
                  (Variables|TilesDimentions|SetWall%20Tile%20Height (.z (.max (StaticMesh|GetBoundingBox _output_get_4))))
                  (bind _returnvalue_4 (AddComponent|AddStaticMeshComponent false (Math|Transform|MakeTransform (Math|Vector|MakeVector (Variables|BuildingSize|GetFinal%20X%20Length) (* (Variables|BuildingSize|GetCurrent%20Y%20Length) -1.0) (Variables|BuildingSize|GetCurrent%20Height)) "0.000000,-90.000000,0.000000" "1.000000,1.000000,1.000000")))
                  (Components|StaticMesh|SetStaticMesh _returnvalue_4 (Variables|Meshes|GetTile)))))
            (Variables|BuildingSize|SetFinal%20Y%20Length (+ (Variables|BuildingSize|GetCurrent%20Y%20Length) (Variables|TilesDimentions|GetWall%20Tile%20Length)))
            (Variables|BuildingSize|SetCurrent%20Y%20Length 0.0)
            (Variables|TilesDimentions|SetWall%20Tile%20Length 0.0))
          (:then_2
            ;[1 1 1] X Back
            (for _index_4 (range 1 (Variables|BuildingSize|GetX%20Size))
              (Variables|BuildingSize|SetX%20Current _index_4)
              (Utilities|FlowControl|Sequence
                (:then_0
                  (Variables|BuildingSize|SetCurrent%20X%20Length (+ (Variables|BuildingSize|GetCurrent%20X%20Length) (Variables|TilesDimentions|GetWall%20Tile%20Length))))
                (:then_1
                  (bind _output_get_5 (Variables|Meshes|SetTile (Utilities|Array|Get(acopy) (select (Utilities|Array|ContainsItem (Variables|DoorsPlacement|GetX%20Door%20Places) (Variables|BuildingSize|GetX%20Current)) (Variables|Meshes|GetWall%202%20Meshes) (Variables|Meshes|GetWall%20Meshes)) (Math|Integer|SelectInt 0 (Math|Integer|SelectInt (Utilities|Array|LastIndex (select (Utilities|Array|ContainsItem (Variables|DoorsPlacement|GetX%20Door%20Places) (Variables|BuildingSize|GetX%20Current)) (Variables|Meshes|GetWall%202%20Meshes) (Variables|Meshes|GetWall%20Meshes))) (Math|Integer|SelectInt (- (Utilities|Array|LastIndex (select (Utilities|Array|ContainsItem (Variables|DoorsPlacement|GetX%20Door%20Places) (Variables|BuildingSize|GetX%20Current)) (Variables|Meshes|GetWall%202%20Meshes) (Variables|Meshes|GetWall%20Meshes))) 1) (Math|Integer|SelectInt (- (Utilities|Array|LastIndex (select (Utilities|Array|ContainsItem (Variables|DoorsPlacement|GetX%20Door%20Places) (Variables|BuildingSize|GetX%20Current)) (Variables|Meshes|GetWall%202%20Meshes) (Variables|Meshes|GetWall%20Meshes))) 2) (Math|Integer|SelectInt (- (Utilities|Array|LastIndex (select (Utilities|Array|ContainsItem (Variables|DoorsPlacement|GetX%20Door%20Places) (Variables|BuildingSize|GetX%20Current)) (Variables|Meshes|GetWall%202%20Meshes) (Variables|Meshes|GetWall%20Meshes))) 3) (Math|Integer|SelectInt (- (Utilities|Array|LastIndex (select (Utilities|Array|ContainsItem (Variables|DoorsPlacement|GetX%20Door%20Places) (Variables|BuildingSize|GetX%20Current)) (Variables|Meshes|GetWall%202%20Meshes) (Variables|Meshes|GetWall%20Meshes))) 3) (Math|Integer|SelectInt (- (Utilities|Array|LastIndex (select (Utilities|Array|ContainsItem (Variables|DoorsPlacement|GetX%20Door%20Places) (Variables|BuildingSize|GetX%20Current)) (Variables|Meshes|GetWall%202%20Meshes) (Variables|Meshes|GetWall%20Meshes))) 4) (Variables|BuildingSize|GetRandom%20Floor) (== (Variables|BuildingSize|GetZ%20Current) (- (Variables|BuildingSize|GetZ%20Floors) 4))) (== (Variables|BuildingSize|GetZ%20Current) (- (Variables|BuildingSize|GetZ%20Floors) 3))) (== (Variables|BuildingSize|GetZ%20Current) (- (Variables|BuildingSize|GetZ%20Floors) 3))) (== (Variables|BuildingSize|GetZ%20Current) (- (Variables|BuildingSize|GetZ%20Floors) 2))) (== (Variables|BuildingSize|GetZ%20Current) (- (Variables|BuildingSize|GetZ%20Floors) 1))) (== (Variables|BuildingSize|GetZ%20Current) (Variables|BuildingSize|GetZ%20Floors))) (== (Variables|BuildingSize|GetZ%20Current) 1)))))
                  (Variables|TilesDimentions|SetWall%20Tile%20Length (.x (.max (StaticMesh|GetBoundingBox _output_get_5))))
                  (Variables|TilesDimentions|SetWall%20Tile%20Height (.z (.max (StaticMesh|GetBoundingBox _output_get_5))))
                  (bind _returnvalue_5 (AddComponent|AddStaticMeshComponent false (Math|Transform|MakeTransform (Math|Vector|MakeVector (+ (Variables|BuildingSize|GetCurrent%20X%20Length) (Variables|TilesDimentions|GetWall%20Tile%20Length)) (* (Variables|BuildingSize|GetFinal%20Y%20Length) -1.0) (Variables|BuildingSize|GetCurrent%20Height)) "0.0,180.000000,0.0" "1.000000,1.000000,1.000000")))
                  (Components|StaticMesh|SetStaticMesh _returnvalue_5 (Variables|Meshes|GetTile)))))
            (Variables|BuildingSize|SetFinal%20X%20Length (+ (Variables|BuildingSize|GetCurrent%20X%20Length) (Variables|TilesDimentions|GetWall%20Tile%20Length)))
            (Variables|BuildingSize|SetCurrent%20X%20Length 0.0)
            (Variables|TilesDimentions|SetWall%20Tile%20Length 0.0))
          (:then_3
            ;[1 1 1] Corners
            (bind _returnvalue_6 (AddComponent|AddStaticMeshComponent false (Math|Transform|MakeTransform (Math|Vector|MakeVector 0.0 0.0 (Variables|BuildingSize|GetCurrent%20Height)) "0, 0, 0" "1.000000,1.000000,1.000000")))
            (Components|StaticMesh|SetStaticMesh _returnvalue_6 (Utilities|Array|Get(acopy) _corner_meshes (Math|Integer|SelectInt 0 (Math|Integer|SelectInt _returnvalue (Math|Integer|SelectInt (- _returnvalue 1) (Math|Integer|SelectInt (- _returnvalue 2) (Math|Integer|SelectInt (- _returnvalue 3) (Math|Integer|SelectInt (- _returnvalue 3) (Math|Integer|SelectInt (- _returnvalue 4) (Variables|BuildingSize|GetRandom%20Floor) (== (Variables|BuildingSize|GetZ%20Current) (- (Variables|BuildingSize|GetZ%20Floors) 4))) (== (Variables|BuildingSize|GetZ%20Current) (- (Variables|BuildingSize|GetZ%20Floors) 3))) (== (Variables|BuildingSize|GetZ%20Current) (- (Variables|BuildingSize|GetZ%20Floors) 3))) (== (Variables|BuildingSize|GetZ%20Current) (- (Variables|BuildingSize|GetZ%20Floors) 2))) (== (Variables|BuildingSize|GetZ%20Current) (- (Variables|BuildingSize|GetZ%20Floors) 1))) (== (Variables|BuildingSize|GetZ%20Current) (Variables|BuildingSize|GetZ%20Floors))) (== (Variables|BuildingSize|GetZ%20Current) 1))))
            (bind _returnvalue_7 (AddComponent|AddStaticMeshComponent false (Math|Transform|MakeTransform (Math|Vector|MakeVector (Variables|BuildingSize|GetFinal%20X%20Length) 0.0 (Variables|BuildingSize|GetCurrent%20Height)) "0.000000,-90.000000,0.000000" "1.000000,1.000000,1.000000")))
            (Components|StaticMesh|SetStaticMesh _returnvalue_7 (Utilities|Array|Get(acopy) _corner_meshes (Math|Integer|SelectInt 0 (Math|Integer|SelectInt _returnvalue (Math|Integer|SelectInt (- _returnvalue 1) (Math|Integer|SelectInt (- _returnvalue 2) (Math|Integer|SelectInt (- _returnvalue 3) (Math|Integer|SelectInt (- _returnvalue 3) (Math|Integer|SelectInt (- _returnvalue 4) (Variables|BuildingSize|GetRandom%20Floor) (== (Variables|BuildingSize|GetZ%20Current) (- (Variables|BuildingSize|GetZ%20Floors) 4))) (== (Variables|BuildingSize|GetZ%20Current) (- (Variables|BuildingSize|GetZ%20Floors) 3))) (== (Variables|BuildingSize|GetZ%20Current) (- (Variables|BuildingSize|GetZ%20Floors) 3))) (== (Variables|BuildingSize|GetZ%20Current) (- (Variables|BuildingSize|GetZ%20Floors) 2))) (== (Variables|BuildingSize|GetZ%20Current) (- (Variables|BuildingSize|GetZ%20Floors) 1))) (== (Variables|BuildingSize|GetZ%20Current) (Variables|BuildingSize|GetZ%20Floors))) (== (Variables|BuildingSize|GetZ%20Current) 1))))
            (bind _returnvalue_8 (AddComponent|AddStaticMeshComponent false (Math|Transform|MakeTransform (Math|Vector|MakeVector 0.0 (* (Variables|BuildingSize|GetFinal%20Y%20Length) -1.0) (Variables|BuildingSize|GetCurrent%20Height)) "0.000000,90.000000,0.000000" "1.000000,1.000000,1.000000")))
            (Components|StaticMesh|SetStaticMesh _returnvalue_8 (Utilities|Array|Get(acopy) _corner_meshes (Math|Integer|SelectInt 0 (Math|Integer|SelectInt _returnvalue (Math|Integer|SelectInt (- _returnvalue 1) (Math|Integer|SelectInt (- _returnvalue 2) (Math|Integer|SelectInt (- _returnvalue 3) (Math|Integer|SelectInt (- _returnvalue 3) (Math|Integer|SelectInt (- _returnvalue 4) (Variables|BuildingSize|GetRandom%20Floor) (== (Variables|BuildingSize|GetZ%20Current) (- (Variables|BuildingSize|GetZ%20Floors) 4))) (== (Variables|BuildingSize|GetZ%20Current) (- (Variables|BuildingSize|GetZ%20Floors) 3))) (== (Variables|BuildingSize|GetZ%20Current) (- (Variables|BuildingSize|GetZ%20Floors) 3))) (== (Variables|BuildingSize|GetZ%20Current) (- (Variables|BuildingSize|GetZ%20Floors) 2))) (== (Variables|BuildingSize|GetZ%20Current) (- (Variables|BuildingSize|GetZ%20Floors) 1))) (== (Variables|BuildingSize|GetZ%20Current) (Variables|BuildingSize|GetZ%20Floors))) (== (Variables|BuildingSize|GetZ%20Current) 1))))
            (bind _returnvalue_9 (AddComponent|AddStaticMeshComponent false (Math|Transform|MakeTransform (Math|Vector|MakeVector (Variables|BuildingSize|GetFinal%20X%20Length) (* (Variables|BuildingSize|GetFinal%20Y%20Length) -1.0) (Variables|BuildingSize|GetCurrent%20Height)) "0.000000,180.000000,0.000000" "1.000000,1.000000,1.000000")))
            (Components|StaticMesh|SetStaticMesh _returnvalue_9 (Utilities|Array|Get(acopy) _corner_meshes (Math|Integer|SelectInt 0 (Math|Integer|SelectInt _returnvalue (Math|Integer|SelectInt (- _returnvalue 1) (Math|Integer|SelectInt (- _returnvalue 2) (Math|Integer|SelectInt (- _returnvalue 3) (Math|Integer|SelectInt (- _returnvalue 3) (Math|Integer|SelectInt (- _returnvalue 4) (Variables|BuildingSize|GetRandom%20Floor) (== (Variables|BuildingSize|GetZ%20Current) (- (Variables|BuildingSize|GetZ%20Floors) 4))) (== (Variables|BuildingSize|GetZ%20Current) (- (Variables|BuildingSize|GetZ%20Floors) 3))) (== (Variables|BuildingSize|GetZ%20Current) (- (Variables|BuildingSize|GetZ%20Floors) 3))) (== (Variables|BuildingSize|GetZ%20Current) (- (Variables|BuildingSize|GetZ%20Floors) 2))) (== (Variables|BuildingSize|GetZ%20Current) (- (Variables|BuildingSize|GetZ%20Floors) 1))) (== (Variables|BuildingSize|GetZ%20Current) (Variables|BuildingSize|GetZ%20Floors))) (== (Variables|BuildingSize|GetZ%20Current) 1)))))))
      (Variables|BuildingSize|SetFinal%20Height (+ (Variables|BuildingSize|GetCurrent%20Height) (Variables|TilesDimentions|GetWall%20Tile%20Height))))
    (:then_1
      (Utilities|FlowControl|Sequence
        (:then_0
          ;[1 1 1] Roof X
          (Variables|BuildingSize|SetCurrent%20Height (+ (Variables|BuildingSize|GetCurrent%20Height) (Variables|TilesDimentions|GetWall%20Tile%20Height)))
          (for _index_5 (range 1 (Variables|BuildingSize|GetX%20Size))
            (Variables|BuildingSize|SetX%20Current _index_5)
            (Utilities|FlowControl|Sequence
              (:then_0
                (Variables|BuildingSize|SetCurrent%20X%20Length (+ (Variables|BuildingSize|GetCurrent%20X%20Length) (Variables|TilesDimentions|GetWall%20Tile%20Length))))
              (:then_1
                (Variables|BuildingSize|SetY%20Current 1)
                (bind _output_get_6 (Variables|Meshes|SetTile (Utilities|Array|Get(acopy) (Variables|Meshes|GetFront%20Roof%20Meshes) (Math|Integer|SelectInt 1 0 (Utilities|Array|ContainsItem (Variables|DoorsPlacement|GetX%20Door%20Places) (Variables|BuildingSize|GetX%20Current))))))
                (Variables|TilesDimentions|SetWall%20Tile%20Length (.x (.max (StaticMesh|GetBoundingBox _output_get_6))))
                (Variables|TilesDimentions|SetWall%20Tile%20Height (.z (.max (StaticMesh|GetBoundingBox _output_get_6))))
                (bind _returnvalue_10 (AddComponent|AddStaticMeshComponent false (Math|Transform|MakeTransform (Math|Vector|MakeVector (Variables|BuildingSize|GetCurrent%20X%20Length) 0.0 (Variables|BuildingSize|GetCurrent%20Height)) "0, 0, 0" "1.000000,1.000000,1.000000")))
                (Components|StaticMesh|SetStaticMesh _returnvalue_10 (Variables|Meshes|GetTile)))
              (:then_2
                (Variables|BuildingSize|SetY%20Current (Variables|BuildingSize|GetY%20Size))
                (bind _output_get_7 (Variables|Meshes|SetTile (Utilities|Array|Get(acopy) (Variables|Meshes|GetFront%20Roof%20Meshes) (Math|Integer|SelectInt 1 0 (Utilities|Array|ContainsItem (Variables|DoorsPlacement|GetX%20Door%20Places) (Variables|BuildingSize|GetX%20Current))))))
                (Variables|TilesDimentions|SetWall%20Tile%20Length (.x (.max (StaticMesh|GetBoundingBox _output_get_7))))
                (Variables|TilesDimentions|SetWall%20Tile%20Height (.z (.max (StaticMesh|GetBoundingBox _output_get_7))))
                (bind _returnvalue_11 (AddComponent|AddStaticMeshComponent false (Math|Transform|MakeTransform (Math|Vector|MakeVector (+ (Variables|BuildingSize|GetCurrent%20X%20Length) (Variables|TilesDimentions|GetWall%20Tile%20Length)) (* (Variables|BuildingSize|GetFinal%20Y%20Length) -1.0) (Variables|BuildingSize|GetCurrent%20Height)) "0.000000,180.000000,0.000000" "1.000000,1.000000,1.000000")))
                (Components|StaticMesh|SetStaticMesh _returnvalue_11 (Variables|Meshes|GetTile)))))
          (Variables|BuildingSize|SetCurrent%20Y%20Length 0.0)
          (Variables|TilesDimentions|SetWall%20Tile%20Length 0.0))
        (:then_1
          ;[1 1 1] Roof Y
          (Variables|BuildingSize|SetCurrent%20Y%20Length -5e+01)
          (for _index_6 (range 1 (Variables|BuildingSize|GetY%20Size))
            (Variables|BuildingSize|SetY%20Current _index_6)
            (Utilities|FlowControl|Sequence
              (:then_0
                (Variables|BuildingSize|SetCurrent%20Y%20Length (+ (Variables|BuildingSize|GetCurrent%20Y%20Length) (Variables|TilesDimentions|GetWall%20Tile%20Length))))
              (:then_1
                (Variables|BuildingSize|SetX%20Current 1)
                (bind _output_get_8 (Variables|Meshes|SetTile (Utilities|Array|Get(acopy) (select (Utilities|Array|ContainsItem (Variables|DoorsPlacement|GetY%20Door%20Places) (Variables|BuildingSize|GetY%20Current)) (Variables|Meshes|GetSide%20Roof%20Meshes%20L) (Variables|Meshes|GetSide%20Roof%20Meshes%20S)) (Math|Integer|SelectInt 2 (Math|Integer|SelectInt 0 1 (or (and (== (Variables|BuildingSize|GetY%20Current) (Variables|BuildingSize|GetY%20Size)) (== (Variables|BuildingSize|GetX%20Current) 1)) (and (== (Variables|BuildingSize|GetY%20Current) 1) (== (Variables|BuildingSize|GetX%20Current) (Variables|BuildingSize|GetX%20Size))))) (or (and (== (Variables|BuildingSize|GetY%20Current) (Variables|BuildingSize|GetY%20Size)) (== (Variables|BuildingSize|GetX%20Current) (Variables|BuildingSize|GetX%20Size))) (and (== (Variables|BuildingSize|GetY%20Current) 1) (== (Variables|BuildingSize|GetX%20Current) 1)))))))
                (Variables|TilesDimentions|SetWall%20Tile%20Length (.x (.max (StaticMesh|GetBoundingBox _output_get_8))))
                (Variables|TilesDimentions|SetWall%20Tile%20Depth (.y (.max (StaticMesh|GetBoundingBox _output_get_8))))
                (Variables|TilesDimentions|SetWall%20Tile%20Height (.z (.max (StaticMesh|GetBoundingBox _output_get_8))))
                (bind _returnvalue_12 (AddComponent|AddStaticMeshComponent false (Math|Transform|MakeTransform (Math|Vector|MakeVector 0.0 (- (* (Variables|BuildingSize|GetCurrent%20Y%20Length) -1.0) (Variables|TilesDimentions|GetWall%20Tile%20Length)) (Variables|BuildingSize|GetCurrent%20Height)) "0.000000,90.000000,0.000000" "1.000000,1.000000,1.000000")))
                (Components|StaticMesh|SetStaticMesh _returnvalue_12 (Variables|Meshes|GetTile)))
              (:then_2
                (Variables|BuildingSize|SetX%20Current (Variables|BuildingSize|GetX%20Size))
                (bind _output_get_9 (Variables|Meshes|SetTile (Utilities|Array|Get(acopy) (select (Utilities|Array|ContainsItem (Variables|DoorsPlacement|GetY%20Door%20Places) (Variables|BuildingSize|GetY%20Current)) (Variables|Meshes|GetSide%20Roof%20Meshes%20L) (Variables|Meshes|GetSide%20Roof%20Meshes%20S)) (Math|Integer|SelectInt 2 (Math|Integer|SelectInt 0 1 (or (and (== (Variables|BuildingSize|GetY%20Current) (Variables|BuildingSize|GetY%20Size)) (== (Variables|BuildingSize|GetX%20Current) 1)) (and (== (Variables|BuildingSize|GetY%20Current) 1) (== (Variables|BuildingSize|GetX%20Current) (Variables|BuildingSize|GetX%20Size))))) (or (and (== (Variables|BuildingSize|GetY%20Current) (Variables|BuildingSize|GetY%20Size)) (== (Variables|BuildingSize|GetX%20Current) (Variables|BuildingSize|GetX%20Size))) (and (== (Variables|BuildingSize|GetY%20Current) 1) (== (Variables|BuildingSize|GetX%20Current) 1)))))))
                (Variables|TilesDimentions|SetWall%20Tile%20Length (.x (.max (StaticMesh|GetBoundingBox _output_get_9))))
                (Variables|TilesDimentions|SetWall%20Tile%20Depth (.y (.max (StaticMesh|GetBoundingBox _output_get_9))))
                (Variables|TilesDimentions|SetWall%20Tile%20Height (.z (.max (StaticMesh|GetBoundingBox _output_get_9))))
                (bind _returnvalue_13 (AddComponent|AddStaticMeshComponent false (Math|Transform|MakeTransform (Math|Vector|MakeVector (Variables|BuildingSize|GetFinal%20X%20Length) (* (Variables|BuildingSize|GetCurrent%20Y%20Length) -1.0) (Variables|BuildingSize|GetCurrent%20Height)) "0.000000,-90.000000,0.000000" "1.000000,1.000000,1.000000")))
                (Components|StaticMesh|SetStaticMesh _returnvalue_13 (Variables|Meshes|GetTile)))))
          (Variables|BuildingSize|SetCurrent%20Y%20Length 0.0)
          (Variables|TilesDimentions|SetWall%20Tile%20Length 0.0)
          (Variables|BuildingSize|SetCurrent%20X%20Length 0.0))
        (:then_2
          ;[1 1 1] Roof Top
          (Variables|BuildingSize|SetCurrent%20Height (+ (Variables|BuildingSize|GetCurrent%20Height) (Variables|TilesDimentions|GetWall%20Tile%20Height)))
          (bind _output_get_10 (Variables|BuildingSize|SetInitial%20roof%20Depth (* (Variables|TilesDimentions|GetWall%20Tile%20Depth) -3.0)))
          (Variables|BuildingSize|SetCurrent%20Y%20Length _output_get_10)
          (Variables|TilesDimentions|SetWall%20Tile%20Depth 0.0)
          (for _index_7 (range 1 (Variables|BuildingSize|GetX%20Size))
            (Variables|BuildingSize|SetX%20Current _index_7)
            (Utilities|FlowControl|Sequence
              (:then_0
                (Variables|BuildingSize|SetCurrent%20X%20Length (+ (Variables|BuildingSize|GetCurrent%20X%20Length) (Variables|TilesDimentions|GetWall%20Tile%20Length))))
              (:then_1
                (for _index_8 (range 1 (Variables|BuildingSize|GetY%20Size))
                  (Variables|BuildingSize|SetY%20Current _index_8)
                  (Utilities|FlowControl|Sequence
                    (:then_0
                      (Variables|BuildingSize|SetCurrent%20Y%20Length (+ (Variables|BuildingSize|GetCurrent%20Y%20Length) (* (Variables|TilesDimentions|GetWall%20Tile%20Depth) -1.0))))
                    (:then_1
                      (bind _output_get_11 (Variables|Meshes|SetTile (Utilities|Array|Get(acopy) (Variables|Meshes|GetTop%20Roof%20Meshes))))
                      (Variables|TilesDimentions|SetWall%20Tile%20Length (* (Math|Float|SelectFloat 1.25 1.0 (Utilities|Array|ContainsItem (Variables|DoorsPlacement|GetX%20Door%20Places) (Variables|BuildingSize|GetX%20Current))) (.x (.max (StaticMesh|GetBoundingBox _output_get_11)))))
                      (Variables|TilesDimentions|SetWall%20Tile%20Depth (* (.x (.max (StaticMesh|GetBoundingBox _output_get_11))) (Math|Float|SelectFloat (Math|Float|SelectFloat 1.0 0.7 (Utilities|Array|ContainsItem (Variables|DoorsPlacement|GetY%20Door%20Places) (Variables|BuildingSize|GetY%20Current))) (Math|Float|SelectFloat 1.25 1.0 (Utilities|Array|ContainsItem (Variables|DoorsPlacement|GetY%20Door%20Places) (Variables|BuildingSize|GetY%20Current))) (or (== (Variables|BuildingSize|GetY%20Current) 1) (== (Variables|BuildingSize|GetY%20Current) (Variables|BuildingSize|GetY%20Size))))))
                      (Variables|TilesDimentions|SetWall%20Tile%20Height (.z (.max (StaticMesh|GetBoundingBox _output_get_11))))
                      (bind _returnvalue_14 (AddComponent|AddStaticMeshComponent false (Math|Transform|MakeTransform (Math|Vector|MakeVector (Variables|BuildingSize|GetCurrent%20X%20Length) (* (Variables|BuildingSize|GetCurrent%20Y%20Length) 1.0) (Variables|BuildingSize|GetCurrent%20Height)) "0, 0, 0" (Math|Vector|MakeVector (Math|Float|SelectFloat 1.25 1.0 (Utilities|Array|ContainsItem (Variables|DoorsPlacement|GetX%20Door%20Places) (Variables|BuildingSize|GetX%20Current))) (Math|Float|SelectFloat (Math|Float|SelectFloat 1.0 0.7 (Utilities|Array|ContainsItem (Variables|DoorsPlacement|GetY%20Door%20Places) (Variables|BuildingSize|GetY%20Current))) (Math|Float|SelectFloat 1.25 1.0 (Utilities|Array|ContainsItem (Variables|DoorsPlacement|GetY%20Door%20Places) (Variables|BuildingSize|GetY%20Current))) (or (== (Variables|BuildingSize|GetY%20Current) 1) (== (Variables|BuildingSize|GetY%20Current) (Variables|BuildingSize|GetY%20Size)))) 1.0))))
                      (Components|StaticMesh|SetStaticMesh _returnvalue_14 (Variables|Meshes|GetTile)))))
                (Variables|BuildingSize|SetCurrent%20Y%20Length (Variables|BuildingSize|GetInitial%20roof%20Depth))
                (Variables|TilesDimentions|SetWall%20Tile%20Depth 0.0)))))))))